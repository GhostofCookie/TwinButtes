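; BP_Tent is an interactable tent that lets the player respawn the clouds by pressing E while overlapping it.
; Overlap events show its widget when a BaseCharacter enters and hide it on exit, while Tick polls for the key press.
; The FadeCamera macro fades the camera out, disables input for a one-second delay, then starts the fade back.
; RespawnClouds then runs on the first CloudArray actor in the level.
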(event Collision|EventActorBeginOverlap
  (params (OtherActor :type Actor%20Object%20Reference))
  ;[0 0 0] Toggle widget
  (Utilities|Casting|CastToBaseCharacter OtherActor)
  (Rendering|SetVisibility (Variables|Default|GetWidget) true false))

(event Collision|EventActorEndOverlap
  (params (OtherActor :type Actor%20Object%20Reference))
  ;[0 0 0] Toggle widget
  (Utilities|Casting|CastToBaseCharacter OtherActor)
  (Rendering|SetVisibility (Variables|Default|GetWidget) false false))

(event EventTick
  (params (DeltaSeconds :type Float%20%28single-precision%29))
  ;[0 0 0] Check if E is pressed. If so, respawn the clouds.
  (if (and (Collision|IsOverlappingActor (Game|Player|GetPlayerPawn 0) :!class /Script/Engine.Actor) (Game|Player|WasInputKeyJustPressed (Game|GetPlayerController 0) "E"))
    (Utilities|FadeCamera
      (:Completed
        (bind _outactors (Actor|GetAllActorsOfClass "/Game/Blueprints/cloudArray/cloudArray.cloudArray_C"))
        (Default|RespawnClouds (Utilities|Array|Get(acopy) _outactors))))))

(fn ConstructionScript)