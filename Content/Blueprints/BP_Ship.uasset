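; Ship actor that sails through BP_Waypoint actors in turn while firing penguin projectiles from its cannons.
; A looping timer drives GoToWayPoint, which turns the ship and runs MoveComponentTo, advancing the index on completion and resetting past the last waypoint.
; Tick stops the move near a waypoint and calls SpawnPenguins, whose Delay paces shots with explosion effects at random left cannons.
; Right cannons are gathered but never fired.
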(event Custom|Move
  (Utilities|GotoWayPoint))

(event EventBeginPlay
  (|SetCannons)
  (Utilities|Time|SetTimerbyEvent (delegate Custom|Move) 0.1 true))

(event EventTick
  (params (DeltaSeconds :type Float%20%28single-precision%29))
  (Utilities|FlowControl|Sequence
    (:then_0
      (Utilities|GotoWayPoint) ; enters at Tick
    )
    (:then_1
      (Utilities|SpawnPenguins))))

(fn ConstructionScript)