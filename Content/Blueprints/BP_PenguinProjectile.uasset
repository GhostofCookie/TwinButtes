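; BP_PenguinProjectile is a projectile that targets the player and does damage on contact.
; On BeginPlay it sets the player BaseCharacter's capsule as the homing target of its ProjectileMovement component.
; When it overlaps the player, it calls AffectHealth on that character with a fixed amount; the graph does not destroy the projectile afterward.
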(event EventBeginPlay
  (bind _asbase_character (Utilities|Casting|CastToBaseCharacter (Game|GetPlayerCharacter 0)))
  (Variables|/Script/Engine.ProjectileMovementComponent|SetHomingTargetComponent (Variables|Default|GetProjectileMovement) (Variables|/Script/Engine.Character|GetCapsuleComponent _asbase_character)))

(event Collision|EventActorBeginOverlap
  (params (OtherActor :type Actor%20Object%20Reference))
  (bind _returnvalue (Game|GetPlayerCharacter 0))
  ;[0 0 0] If it overlaps the player, do damage
  (if (== OtherActor _returnvalue)
    (bind _asbase_character (Utilities|Casting|CastToBaseCharacter _returnvalue))
    (Class|BaseCharacter|AffectHealth _asbase_character 1e+02)))

(fn ConstructionScript)