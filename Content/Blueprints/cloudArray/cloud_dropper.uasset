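; Cloud dropper is a cloud platform that fades and shifts vertically when the player character overlaps its collider.
; A Dissipate timeline drives the dynamic material's opacityMax and offsets the mesh's height with sweep.
; At zero opacity it disables collision, waits briefly, then runs RestoreCloud to bring back opacity and re-enable collision.
; Ending the overlap jumps straight to that restore, which leaves height unchanged.
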(event OnComponentBeginOverlap(collider)
  (params (OverlappedComponent :type Primitive%20Component%20Object%20Reference) (OtherActor :type Actor%20Object%20Reference) (OtherComp :type Primitive%20Component%20Object%20Reference) (OtherBodyIndex :type Integer) (bFromSweep :type Boolean) (SweepResult :type Hit%20Result%20Structure%20%28by%20ref%29))
  (bind _cloud (Variables|Default|Getcloud))
  (bind _returnvalue (Transformation|GetWorldLocation _cloud))
  (if (== OtherActor (Variables|Default|GetCharacter))
    ;[0 0 0] Dissipate cloud over time if overlapping
    (bind (_direction _opacity _cloudheight) (Timeline|Dissipate PlayFromStart)
      (:Update
        (Rendering|Material|SetScalarParameterValue (Variables|Default|GetCloudMaterial) "opacityMax" _opacity :!class /Script/Engine.MaterialInstanceDynamic)
        (Transformation|SetWorldLocation _cloud (Math|Vector|MakeVector (.x _returnvalue) (.y _returnvalue) (+ (.z _cloudheight) (.z _returnvalue))) true false))
      (:Finished
        (if (== _opacity 0.0)
          (Collision|SetCollisionEnabled _cloud "NoCollision")
          (Utilities|FlowControl|Delay 1.0)
          (bind _returnvalue_2 (Rendering|Material|GetScalarParameterValue (Variables|Default|GetCloudMaterial) "opacityMax" :!class /Script/Engine.MaterialInstanceDynamic))
          ;[0 0 0] Restore cloud over time
          (bind _opactity (Timeline|RestoreCloud Play)
            (:Update
              (Rendering|Material|SetScalarParameterValue (Variables|Default|GetCloudMaterial) "opacityMax" _opactity :!class /Script/Engine.MaterialInstanceDynamic))
            (:Finished
              (Collision|SetCollisionEnabled (Variables|Default|Getcloud) "QueryAndPhysics"))))))))

(event OnComponentEndOverlap(collider)
  (params (OverlappedComponent :type Primitive%20Component%20Object%20Reference) (OtherActor :type Actor%20Object%20Reference) (OtherComp :type Primitive%20Component%20Object%20Reference) (OtherBodyIndex :type Integer))
  (if (== OtherActor (Variables|Default|GetCharacter))
    (bind _returnvalue (Rendering|Material|GetScalarParameterValue (Variables|Default|GetCloudMaterial) "opacityMax" :!class /Script/Engine.MaterialInstanceDynamic))
    ;[0 0 0] Restore cloud over time
    (bind _opactity (Timeline|RestoreCloud Play)
      (:Update
        (Rendering|Material|SetScalarParameterValue (Variables|Default|GetCloudMaterial) "opacityMax" _opactity :!class /Script/Engine.MaterialInstanceDynamic))
      (:Finished
        (Collision|SetCollisionEnabled (Variables|Default|Getcloud) "QueryAndPhysics")))))

(event EventBeginPlay
  (|CallParentFunction)
  (bind _returnvalue (Rendering|Material|CreateDynamicMaterialInstance (Variables|Default|Getcloud) 0 "/Game/Materials/M_cloud_dropper.M_cloud_dropper" "None" :!class /Script/Engine.PrimitiveComponent))
  (Variables|Default|SetCloudMaterial _returnvalue)
  ;[0 0 0] Get character information
  (bind _asbase_character (Utilities|Casting|CastToBaseCharacter (Game|Player|GetPlayerPawn 0))
    (:then
      (Variables|Default|SetCharacter _asbase_character))
    (:CastFailed
      (Development|PrintString "No Character!"))))

(fn ConstructionScript
  (|CallParentFunction))