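; Decorative cloud array actor that scatters non-colliding clouds in a field around itself on BeginPlay.
; SpawnField walks a square grid centred on the actor and randomly fills cells based on CloudChance.
; SpawnCloud places a Cloud_basic with grid spacing, random height offset, rotation and scale, then disables its collision.
; A leftover 90% random branch has no effect, and the Cloud_dropper spawn path never runs.
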(event EventBeginPlay
  (CallFunction|SpawnField))

(fn ConstructionScript)

(fn RandomScale
  (bind _cloudmaxscaley (Variables|Default|GetcloudMaxScaleY))
  (bind _cloudmaxscalez (Variables|Default|GetcloudMaxScaleZ))
  (bind _cloudmaxscalex (Variables|Default|GetcloudMaxScaleX))
  (return (Math|Random|RandomFloatinRange (/ _cloudmaxscalex 2.0) _cloudmaxscalex) (Math|Random|RandomFloatinRange (/ _cloudmaxscaley 2.0) _cloudmaxscaley) (Math|Random|RandomFloatinRange (/ _cloudmaxscalez 2.0) _cloudmaxscalez)))

(fn RandomRotation
  (bind _cloudmaxrotationx (Variables|Default|GetcloudMaxRotationX))
  (bind _cloudmaxrotationy (Variables|Default|GetcloudMaxRotationY))
  (bind _cloudmaxrotationz (Variables|Default|GetcloudMaxRotationZ))
  (return (Math|Random|RandomFloatinRange (* _cloudmaxrotationx -1.0) _cloudmaxrotationx) (Math|Random|RandomFloatinRange (* _cloudmaxrotationy -1.0) _cloudmaxrotationy) (Math|Random|RandomFloatinRange (* _cloudmaxrotationz -1.0) _cloudmaxrotationz)))

(fn GetDistance
  (params (X :type Integer) (Y :type Integer))
  (bind _returnvalue (Transformation|GetActorLocation))
  (bind _clouddistancez (Variables|Default|GetcloudDistanceZ))
  (bind _clouddistancexy (Variables|Default|GetcloudDistanceXY))
  ;[0 0 0] distance each cloud is spread
  (return (Math|Vector|MakeVector (+ (.x _returnvalue) (* X _clouddistancexy)) (+ (.y _returnvalue) (* Y _clouddistancexy)) (+ (.z _returnvalue) (Math|Random|RandomFloatinRange (* _clouddistancez -1.0) _clouddistancez)))))

(fn SpawnField
  (bind _cloudnum (Variables|Default|GetcloudNum))
  (bind _cloudnum_2 (Variables|Default|GetcloudNum))
  (bind _index (Utilities|FlowControl|ForLoopwithBreak (/ (* _cloudnum_2 -1) 2) (- (/ _cloudnum_2 2) 1))
    (:LoopBody
      (Variables|Default|SetidxY _index)
      (bind _index_2 (Utilities|FlowControl|ForLoopwithBreak (/ (* _cloudnum -1) 2) (- (/ _cloudnum 2) 1))
        (:LoopBody
          (Variables|Default|SetidxX _index_2)
          (if (== (Math|Random|RandomIntegerinRange 0 (Variables|Default|GetcloudChance)) 0)
            (CallFunction|SpawnCloud (Variables|Default|GetidxX) (Variables|Default|GetidxY))))))))

(fn SpawnCloud
  (params (X :type Integer) (Y :type Integer))
  ;[0 0 0] For Single Path
  (bind _location (CallFunction|GetDistance X Y))
  (LocalVariables|SetLocation _location)
  (bind (_rotx _roty _rotz) (CallFunction|RandomRotation))
  (LocalVariables|SetRotation (Math|Rotator|MakeRotator _rotx _roty _rotz))
  (bind (_scalex _scaley _scalez) (CallFunction|RandomScale))
  (LocalVariables|SetScale (Math|Vector|MakeVector _scalex _scaley _scalez))
  (if (< (Math|Random|RandomFloatinRange 0.0 1.0) 0.9)
    _
    (else
      _))
  (bind _returnvalue (Game|SpawnActorfromClass "/Game/Blueprints/cloudArray/cloud_basic.cloud_basic_C" (Math|Transform|MakeTransform (LocalVariables|GetLocation) (LocalVariables|GetRotation) (LocalVariables|GetScale)) "AdjustIfPossibleButAlwaysSpawn" 0 0))
  (Collision|SetCollisionEnabled (Variables|/Game/Blueprints/cloudArray/cloud.cloud_C|Getcloud _returnvalue) "NoCollision"))