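; Thundercloud actor that randomly flashes a lightning bolt and damages the player standing in its strike area.
; Each Tick yaw-billboards the bolt toward the player's camera and rolls a random integer between Min and Max, striking on zero.
; A strike briefly shows the bolt, removing health if LightningCollision overlap events have flagged the player.
; Hiding the bolt also clears that overlap flag.
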(event OnComponentBeginOverlap(LightningCollision)
  (params (OverlappedComponent :type Primitive%20Component%20Object%20Reference) (OtherActor :type Actor%20Object%20Reference) (OtherComp :type Primitive%20Component%20Object%20Reference) (OtherBodyIndex :type Integer) (bFromSweep :type Boolean) (SweepResult :type Hit%20Result%20Structure%20%28by%20ref%29))
  (if (== OtherActor (Variables|Default|GetCharacter))
    (Variables|Default|SetOverlap true)))

(event OnComponentEndOverlap(LightningCollision)
  (params (OverlappedComponent :type Primitive%20Component%20Object%20Reference) (OtherActor :type Actor%20Object%20Reference) (OtherComp :type Primitive%20Component%20Object%20Reference) (OtherBodyIndex :type Integer))
  (if (== OtherActor (Variables|Default|GetCharacter))
    (Variables|Default|SetOverlap false)))

(event EventBeginPlay
  (CallFunction|LightningStrikeOff)
  (bind _asbase_character (Utilities|Casting|CastToBaseCharacter (Game|Player|GetPlayerPawn 0))
    (:then
      (Variables|Default|SetCharacter _asbase_character))
    (:CastFailed
      (Development|PrintString "No Character!"))))

(event EventTick
  (params (DeltaSeconds :type Float%20%28single-precision%29))
  (bind _lightning (Variables|Default|GetLightning))
  (bind _returnvalue (Transformation|GetWorldRotation _lightning))
  (Transformation|SetWorldRotation _lightning (Math|Rotator|MakeRotator (.roll _returnvalue) (.pitch _returnvalue) (+ (.yaw (Math|Rotator|FindLookatRotation (Transformation|GetWorldLocation _lightning) (Transformation|GetWorldLocation (Variables|/Script/TwinButtes.BaseCharacter|GetCameraComponent (Variables|Default|GetCharacter))))) 9e+01)) false false)
  (bind _strike_ (CallFunction|StrikeChance))
  (if _strike_
    ;[0 0 0] Strike the player
    (CallFunction|LightningStrikeon)
    (Utilities|FlowControl|Delay 0.2)
    (CallFunction|LightningStrikeOff)))

(fn ConstructionScript
  (|CallParentFunction))

(fn StrikeChance
  (return (== (Math|Random|RandomIntegerinRange (LocalVariables|Getmin) (LocalVariables|Getmax)) 0)))

(fn LightningStrikeon
  (Rendering|SetVisibility (Variables|Default|GetLightning) true false)
  (if (Variables|Default|GetOverlap)
    (Class|BaseCharacter|AffectHealth (Variables|Default|GetCharacter) 5e+01)
    (Development|PrintString "Hit by Lightning: -50HP")))

(fn LightningStrikeOff
  (Rendering|SetVisibility (Variables|Default|GetLightning) false false)
  (Variables|Default|SetOverlap false))