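; Cloud array actor that scatters randomly varied clouds over a flat grid centred on its own location at BeginPlay.
; Nested X/Y loops give each cell a random chance to spawn a cloud, spaced by CloudDistance, and end each row early once its cloud cap is reached.
; Helper functions randomise rotation and scale, colliding spawns are skipped, and results are stored in the Clouds array.
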(event EventBeginPlay
  (bind _returnvalue (Transformation|GetActorLocation))
  (bind _clouddistance (Variables|Default|GetcloudDistance))
  ;[0 0 0] Helps spawn objects along an array while centering around origin
  (bind _index (Utilities|FlowControl|ForLoopwithBreak (/ (* (Variables|Default|GetcloudNumY) -1) 2) (/ (Variables|Default|GetcloudNumY) 2))
    (:LoopBody
      (Variables|Default|SetidxY _index)
      (bind _index_2 (Utilities|FlowControl|ForLoopwithBreak (/ (* (Variables|Default|GetcloudNumX) -1) 2) (/ (Variables|Default|GetcloudNumX) 2) :!label _label)
        (:LoopBody
          (Variables|Default|SetidxX _index_2)
          (if (< (Variables|Default|GetnumOnRows) (Variables|Default|GetmaxNumOnRows))
            (if (== (Math|Random|RandomIntegerinRange 0 (Variables|Default|GetcloudSpawnChance%280-n%29)) 0)
              (Math|Integer|IncrementInt (Variables|Default|GetnumOnRows)
                (:%20%20
                  (bind (_rotx _roty _rotz) (CallFunction|RandomRotation))
                  (bind (_scalex _scaley _scalez) (CallFunction|RandomScale))
                  (bind _returnvalue_2 (Game|SpawnActorfromClass "/Game/Blueprints/cloudArray/cloud.cloud_C" (Math|Transform|MakeTransform (Math|Vector|MakeVector (+ (.x _returnvalue) (* (Variables|Default|GetidxX) _clouddistance)) (+ (.y _returnvalue) (* (Variables|Default|GetidxY) _clouddistance)) (.z _returnvalue)) (Math|Rotator|MakeRotator _rotx _roty _rotz) (Math|Vector|MakeVector _scalex _scaley _scalez)) "DontSpawnIfColliding" 0 0))
                  (Utilities|Array|Add (Variables|Default|Getclouds) _returnvalue_2))))
            (else
              (Variables|Default|SetnumOnRows 0)
              (goto _label Break))))
        (:Completed
          (Variables|Default|SetnumOnRows 0))))))

(fn ConstructionScript)

(fn RandomScale
  (bind _cloudmaxscaley (Variables|Default|GetcloudMaxScaleY))
  (bind _cloudmaxscalez (Variables|Default|GetcloudMaxScaleZ))
  (bind _cloudmaxscalex (Variables|Default|GetcloudMaxScaleX))
  (return (Math|Random|RandomFloatinRange (/ _cloudmaxscalex 2.0) _cloudmaxscalex) (Math|Random|RandomFloatinRange (/ _cloudmaxscaley 2.0) _cloudmaxscaley) (Math|Random|RandomFloatinRange (/ _cloudmaxscalez 2.0) _cloudmaxscalez)))

(fn RandomRotation
  (bind _cloudmaxrotationx (Variables|Default|GetcloudMaxRotationX))
  (bind _cloudmaxrotationy (Variables|Default|GetcloudMaxRotationY))
  (bind _cloudmaxrotationz (Variables|Default|GetcloudMaxRotationZ))
  (return (Math|Random|RandomFloatinRange (* _cloudmaxrotationx -1.0) _cloudmaxrotationx) (Math|Random|RandomFloatinRange (* _cloudmaxrotationy -1.0) _cloudmaxrotationy) (Math|Random|RandomFloatinRange (* _cloudmaxrotationz -1.0) _cloudmaxrotationz)))